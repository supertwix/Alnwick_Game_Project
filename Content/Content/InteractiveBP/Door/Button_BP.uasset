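; Interactable button that opens every Door_BP whose DoorID matches its SwitchID and closes all other doors in the level.
; A box trigger adds an InteractPrompt widget while a ThirdPersonCharacter overlaps it and removes it on exit.
; Interact plays a lever sound, briefly flags the prompt as pressed, then updates the doors.
; Inside that door loop it disables the box's overlap events and removes the prompt, with no re-enable here.
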(event `/Game/InteractiveBP/Door/ButtonInterface_BP.Interact`
  ;[1 1 1] Changes the isPressed variable to change the colour of the widget
  (`GameplayStatics.PlaySoundAtLocation` "/Game/Sounds/Environment/lever_big_1.lever_big_1" (`self.K2_GetActorLocation`) (struct) 1.0 1.0 0.0 null null null)
  (set `/Game/InteractiveBP/Door/InteractPrompt.IsPressed` true (stale `self.Box.OnComponentBeginOverlap` _returnvalue))
  (`KismetSystemLibrary.Delay` 0.2)
  (set `/Game/InteractiveBP/Door/InteractPrompt.IsPressed` false (stale `self.Box.OnComponentBeginOverlap` _returnvalue))
  ;[1 1 1] Finds all doors in the level, if the Doors ID matches the switch it will run the doors open function otherwise it will close the door
  (bind _outactors (`GameplayStatics.GetAllActorsOfClass` "/Game/InteractiveBP/Door/Door_BP.Door_BP_C"))
  (for _array_element _outactors
    (if (== (`/Game/InteractiveBP/Door/Door_BP.DoorID` _array_element) (`self.SwitchID`))
      ;;[1 1 1] Sets the box component to be unable to generate overlap events and removes the interact widget
      (`/Game/InteractiveBP/Door/Door_BP.Open Door` _array_element)
      (else
        (`/Game/InteractiveBP/Door/Door_BP.Close Door` _array_element)))
    (set `PrimitiveComponent.bGenerateOverlapEvents` false (`self.Box`))
    ;[1 1 1] Creates the interact prompt widget when the player ooverlaps the button and removes it when they stop
    (`Widget.RemoveFromParent` (stale `self.Box.OnComponentBeginOverlap` _returnvalue) :!label _label)))

(event `self.Box.OnComponentBeginOverlap`
  (params (OverlappedComponent :type "PrimitiveComponent Object Reference") (OtherActor :type "Actor Object Reference") (OtherComp :type "PrimitiveComponent Object Reference") (OtherBodyIndex :type Integer) (bFromSweep :type Boolean) (SweepResult :type "HitResult Structure (by ref)"))
  ;[1 1 1] Creates the interact prompt widget when the player ooverlaps the button and removes it when they stop
  (cast `/Game/ThirdPersonBP/Blueprints/ThirdPersonCharacter` OtherActor)
  (bind _returnvalue (`|CreateWidget` "/Game/InteractiveBP/Door/InteractPrompt.InteractPrompt_C"))
  (`UserWidget.AddToViewport` _returnvalue 0))

(event `self.Box.OnComponentEndOverlap`
  (params (OverlappedComponent :type "PrimitiveComponent Object Reference") (OtherActor :type "Actor Object Reference") (OtherComp :type "PrimitiveComponent Object Reference") (OtherBodyIndex :type Integer))
  ;[1 1 1] Creates the interact prompt widget when the player ooverlaps the button and removes it when they stop
  (cast `/Game/ThirdPersonBP/Blueprints/ThirdPersonCharacter` OtherActor)
  (goto _label))

(fn `UserConstructionScript`)