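; Fire trap Blueprint that cycles a fire particle effect on and off and damages actors caught in it.
; A one-shot timer at BeginPlay starts SetFire, which loops through delays set by OnTime and OffTime, playing a sound at each ignition.
; Overlap events track contact, damaging an actor that enters active fire.
; If anything is overlapping at ignition, the player pawn takes the damage.
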(event `self.ReceiveActorEndOverlap`
  (params (OtherActor :type "Actor Object Reference"))
  (set `self.overlapped` false))

(event `self.ReceiveActorBeginOverlap`
  (params (OtherActor :type "Actor Object Reference"))
  ;[1 1 1] Applies damage if player is still overlapped with triggerbox once fire starts up again
  (set `self.overlapped` true)
  (if (`self.fireOn`)
    (`GameplayStatics.ApplyDamage` OtherActor 1.0 null self)))

(event `SetFire`
  ;[1 1 1] Sets timer to activate, and does damage if contact with fire
  (`ActorComponent.Activate` (`self.ParticleSystem`) false :!label _label)
  (`GameplayStatics.PlaySoundAtLocation` "/Game/Sounds/Environment/FireCue.FireCue" (`SceneComponent.K2_GetComponentLocation` (`self.Cube`)) (struct) 1.0 1.0 0.0 null null null)
  (if (`self.overlapped`)
    (`GameplayStatics.ApplyDamage` (`GameplayStatics.GetPlayerPawn` 0) 1.0 null self))
  (set `self.fireOn` true)
  (`KismetSystemLibrary.Delay` (`self.OnTime`))
  (`ActorComponent.Deactivate` (`self.ParticleSystem`))
  (set `self.fireOn` false)
  (`KismetSystemLibrary.Delay` (`self.OffTime`))
  (goto _label))

(event `self.ReceiveBeginPlay`
  (`KismetSystemLibrary.K2_SetTimer` null "SetFire" 6.0))

(fn `UserConstructionScript`)