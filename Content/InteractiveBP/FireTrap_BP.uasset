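; FireTrap_BP is a timed fire hazard that cycles a particle flame on and off and damages what touches it.
; BeginPlay starts SetFire after an initial timer, which then loops itself through Delays, burning briefly and resting longer.
; Actors entering during a burn take one small hit.
; At ignition, an overlap flag triggers damage to the player pawn, whichever actor set it.
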(event `self.ReceiveActorEndOverlap`
  (params (OtherActor :type "Actor Object Reference"))
  (set `self.overlapped` false))

(event `self.ReceiveActorBeginOverlap`
  (params (OtherActor :type "Actor Object Reference"))
  (set `self.overlapped` true)
  (if (`self.fireOn`)
    (`GameplayStatics.ApplyDamage` OtherActor 0.33)))

(event `SetFire`
  (`ActorComponent.Activate` (`self.ParticleSystem`) false :!label _label)
  (if (`self.overlapped`)
    (`GameplayStatics.ApplyDamage` (`GameplayStatics.GetPlayerPawn` 0) 0.33))
  (set `self.fireOn` true)
  (`KismetSystemLibrary.Delay` 3.0)
  (`ActorComponent.Deactivate` (`self.ParticleSystem`))
  (set `self.fireOn` false)
  (`KismetSystemLibrary.Delay` 6.0)
  (goto _label))

(event `self.ReceiveBeginPlay`
  (`KismetSystemLibrary.K2_SetTimer` null "SetFire" 6.0))

(fn `UserConstructionScript`)