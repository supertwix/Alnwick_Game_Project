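; Speed power-up pickup that boosts the player's movement when overlapped.
; On overlap it raises the Third Person Character's max walk speed and acceleration and plays a teleport sound, with no revert of the boost in this graph.
; It then hides itself and disables its sphere collision, and after a short delay reappears and re-enables collision to respawn.
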(event `self.ReceiveActorBeginOverlap`
  (params (OtherActor :type "Actor Object Reference"))
  (bind _asthird_person_character (cast `/Game/ThirdPersonBP/Blueprints/ThirdPersonCharacter` (`GameplayStatics.GetPlayerCharacter` 0)))
  (bind _charactermovement (`Character.CharacterMovement` _asthird_person_character))
  (set `CharacterMovementComponent.MaxWalkSpeed` 1500.0 _charactermovement)
  (set `CharacterMovementComponent.MaxAcceleration` 4000.0 _charactermovement)
  (`GameplayStatics.PlaySoundAtLocation` "/Engine/VREditor/Sounds/VR_teleport.VR_teleport" (0.0 0.0 0.0) (struct) 0.6 1.0 0.0 null null null)
  ;[1 1 1] Makes power up respawn after 2 seconds
  (`self.SetActorHiddenInGame` true)
  (`PrimitiveComponent.SetCollisionEnabled` (`self.Sphere1`) "NoCollision")
  (`KismetSystemLibrary.Delay` 2.0)
  (`self.SetActorHiddenInGame` false)
  (`PrimitiveComponent.SetCollisionEnabled` (`self.Sphere1`) "QueryAndPhysics"))

(fn `UserConstructionScript`)