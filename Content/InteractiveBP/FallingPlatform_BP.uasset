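; FallingPlatform_BP is an interactive platform that sinks when an actor overlaps it, then rises back.
; BeginPlay caches the world locations of the Origin and SunkAnchor components as endpoints.
; An overlap while at the origin plays a timeline that lerps the actor between them.
; On finish, the timeline reverses if the mesh is away from the origin, so position checks serve as the state.
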(event `self.ReceiveBeginPlay`
  (set `self.OriginVector` (`SceneComponent.K2_GetComponentLocation` (`self.Origin`)))
  (set `self.SunkVector` (`SceneComponent.K2_GetComponentLocation` (`self.SunkAnchor`))))

(event `self.ReceiveActorBeginOverlap`
  (params (OtherActor :type "Actor Object Reference"))
  (bind _returnvalue (== (`self.OriginVector`) (`SceneComponent.K2_GetComponentLocation` (`self.StaticMeshComponent`))))
  (if _returnvalue
    (bind (_direction _sink) (`Timeline|Timeline_0` :!via `PlayFromStart` :!label _label)
      (:`Update`
        (`self.K2_SetActorLocation` (`KismetMathLibrary.VLerp` (`self.OriginVector`) (`self.SunkVector`) _sink)))
      (:`Finished`
        (if (not _returnvalue)
          (goto _label :!via `ReverseFromEnd`))))))

(fn `UserConstructionScript`)